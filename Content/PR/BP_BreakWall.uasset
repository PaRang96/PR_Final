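; BP_BreakWall is a breakable wall that awards points to the runner who destroys it.
; AnyDamage lowers HP; at zero it casts the DamageCauser to RunCharacter, adds points through BP_RunPlayerState, plays hit effect and explosion sound at that character, then destroys itself.
; BreakWallFunc spawns the same effects at the wall's mesh but is not called here.
; An attack-dispatcher binding path is left unconnected.
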(event `self.ReceiveAnyDamage`
  (params (Damage :type "Float (single-precision)") (DamageType :type "DamageType Object Reference") (InstigatedBy :type "Controller Object Reference") (DamageCauser :type "Actor Object Reference"))
  ;[1 1 1] 이 부분은 우선 보류
  (bind _output_get (set `self.HP` (- (`self.HP`) Damage)))
  (if (<= _output_get 0.0)
    (bind _asrun_character (cast `/Game/PR/PlayerCharacter/RunCharacter` DamageCauser))
    (bind _asbp_run_player_state (cast `/Game/PR/GameMode/RunGame/BP_RunPlayerState` (`Pawn.PlayerState` _asrun_character)))
    (`/Game/PR/GameMode/RunGame/BP_RunPlayerState.AddPoint` _asbp_run_player_state 300)
    (bind _returnvalue (`self.K2_GetActorLocation` _asrun_character))
    (`NiagaraFunctionLibrary.SpawnSystemAtLocation` "/Game/PR/VFX/NS_BasicHit.NS_BasicHit" _returnvalue)
    (`GameplayStatics.PlaySoundAtLocation` "/Game/StarterContent/Audio/Explosion_Cue.Explosion_Cue" _returnvalue (struct) 1.0 1.0 0.0 null null null)
    (`self.K2_DestroyActor`)))

(fn `BreakWallFunc`
  (locals (ActorLocation :type "Vector Structure" :default (0.0 0.0 0.0)))
  (bind _output_get (set `local.ActorLocation` (`SceneComponent.K2_GetComponentLocation` (`self.StaticMesh`))))
  (`NiagaraFunctionLibrary.SpawnSystemAtLocation` "/Game/PR/VFX/NS_BasicHit.NS_BasicHit" _output_get)
  (`GameplayStatics.PlaySoundAtLocation` "/Game/StarterContent/Audio/Explosion_Cue.Explosion_Cue" (`local.ActorLocation`) (struct) 1.0 1.0 0.0 null null null))

(fn `UserConstructionScript`)