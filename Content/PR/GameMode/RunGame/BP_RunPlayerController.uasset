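; Player controller for the Run game mode, linking the player's game instance data, player state and HUD.
; On possess, it reads slot and name from RunGI and passes them through Req/Res events into BP_RunPlayerState.
; Finish events forward the finished-player value to BP_RunHUD to update the finish number.
; SendDisableMovement deactivates the InheritRunCharacter's movement and switches to UI-only input with a visible cursor.
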(event `ReqFinishPlayer`
  (params (FinishedPlayer :type Integer))
  (`self.ResFinishPlayer` FinishedPlayer))

(event `ResFinishPlayer`
  (params (`Finished Player` :type Integer))
  (bind _asbp_run_hud (cast `/Game/PR/Widget/Run/BP_RunHUD` (`self.GetHUD`)))
  (`/Game/PR/Widget/Run/BP_RunHUD.UpdateFinishNumber` _asbp_run_hud `Finished Player`))

(event `self.ReceivePossess`
  (params (PossessedPawn :type "Pawn Object Reference"))
  (`self.ResClientPossess`)
  (`self.ResUpdateName`))

(event `ResClientPossess`
  (bind _asrun_gi (cast `/Game/PR/GameMode/RunGI` (`GameplayStatics.GetGameInstance`)))
  (`self.ReqSetPlayerNumber` (`/Game/PR/GameMode/RunGI.Slots` _asrun_gi)))

(event `ResUpdateName`
  (bind _asrun_gi (cast `/Game/PR/GameMode/RunGI` (`GameplayStatics.GetGameInstance`)))
  (`self.ReqUpdateName` (`/Game/PR/GameMode/RunGI.Name` _asrun_gi)))

(event `ReqSetPlayerNumber`
  (params (PlayerNumber :type Integer))
  (bind _asbp_run_player_state (cast `/Game/PR/GameMode/RunGame/BP_RunPlayerState` (`self.PlayerState`)))
  (`/Game/PR/GameMode/RunGame/BP_RunPlayerState.Get Player Number` _asbp_run_player_state PlayerNumber))

(event `ReqUpdateName`
  (params (Name :type String))
  (bind _asbp_run_player_state (cast `/Game/PR/GameMode/RunGame/BP_RunPlayerState` (`self.PlayerState`)))
  (`/Game/PR/GameMode/RunGame/BP_RunPlayerState.SetName` _asbp_run_player_state Name))

(event `SendDisableMovement`
  (`self.DisableMovement`)
  (`WidgetBlueprintLibrary.SetInputMode_UIOnlyEx` self null)
  (set `self.bShowMouseCursor` true))

(fn `DisableMovement`
  (bind _asinherit_run_character (cast `/Game/PR/PlayerCharacter/InheritRunCharacter` (`self.K2_GetPawn`)))
  (`ActorComponent.Deactivate` (`Character.CharacterMovement` _asinherit_run_character)))

(fn `UserConstructionScript`)