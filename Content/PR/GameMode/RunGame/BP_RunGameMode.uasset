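; Game mode for the Run race game, moving a match from waiting for players through racing and finish to the scoreboard.
; Tick polls the state enum on RunGS: play starts when player count matches the game instance's Slots, and finish begins once BP_Goal records a player.
; After a one-minute delay, the final state creates and displays a new Scoreboard_Widget on every tick.
; Input-disabling logic is present but unconnected.
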(event `self.ReceiveBeginPlay`
  (set `/Game/PR/GameMode/RunGS.EN_GameState` "NewEnumerator0" (`self.GetRunGameState`)))

(event `self.ReceiveTick`
  (params (DeltaSeconds :type "Float (single-precision)"))
  (bind _asrun_game_state (`self.GetRunGameState`))
  (bind _asrun_game_state_2 (`self.GetRunGameState`))
  (`|ExecutionSequence`
    (:`then_0`
      (if (`|EnumEquality` (`/Game/PR/GameMode/RunGS.EN_GameState` (`self.GetRunGameState`)) "NewEnumerator0")
        (bind _asrun_gi (cast `/Game/PR/GameMode/RunGI` (`GameplayStatics.GetGameInstance`)))
        (bind _returnvalue (`self.GetNumPlayers`))
        (if (== _returnvalue (`/Game/PR/GameMode/RunGI.Slots` _asrun_gi))
          (set `/Game/PR/GameMode/RunGS.EN_GameState` "NewEnumerator1" (`self.GetRunGameState`)))))
    (:`then_1`
      (if (`|EnumEquality` (`/Game/PR/GameMode/RunGS.EN_GameState` _asrun_game_state_2) "NewEnumerator1")
        (if (`self.FirstPlayerPassed`)
          (set `/Game/PR/GameMode/RunGS.EN_GameState` "NewEnumerator2" _asrun_game_state_2)
          (`KismetSystemLibrary.PrintString` "Game State: Finish" true true (struct :`R` 0.117151 :`G` 0.173611 :`B` 0.110445 :`A` 1.0) 50.0))))
    (:`then_2`
      (if (`|EnumEquality` (`/Game/PR/GameMode/RunGS.EN_GameState` _asrun_game_state) "NewEnumerator2")
        (`KismetSystemLibrary.Delay` 60.0)
        (set `/Game/PR/GameMode/RunGS.EN_GameState` "NewEnumerator3" _asrun_game_state)))
    (:`then_3`
      (if (`|EnumEquality` (`/Game/PR/GameMode/RunGS.EN_GameState` (`self.GetRunGameState`)) "NewEnumerator3")
        (bind _returnvalue_2 (`|CreateWidget` "/Game/PR/Widget/Run/Scoreboard_Widget.Scoreboard_Widget_C"))
        (`/Game/PR/Widget/Run/Scoreboard_Widget.UpdateScoreboard` _returnvalue_2)
        (`UserWidget.AddToViewport` _returnvalue_2 0)))))

(event `SendScoreboard`
  (params (Scoreboard :type "/Game/PR/Widget/Run/Scoreboard_Widget Object Reference"))
  (`self.RecvScoreboard` Scoreboard))

(event `RecvScoreboard`
  (params (Scoreboard :type "/Game/PR/Widget/Run/Scoreboard_Widget Object Reference"))
  (`UserWidget.AddToViewport` Scoreboard 0))

(fn `FirstPlayerPassed`
  (returns (FirstPlaceFilled :type Boolean))
  (bind _returnvalue (`GameplayStatics.GetActorOfClass` "/Game/PR/ActorBlueprints/BP_Goal.BP_Goal_C"))
  (return (> (`KismetArrayLibrary.Array_Length` (`/Game/PR/ActorBlueprints/BP_Goal.PlayerRankingController` _returnvalue)) 0)))

(fn `GetAllPlayerControllers`
  (returns (`AsBP Run Player Controller` :type "/Game/PR/GameMode/RunGame/BP_RunPlayerController Object Reference"))
  (bind _returnvalue (`self.GetNumPlayers`))
  (for _index (range _returnvalue)
    (bind _asbp_run_player_controller (cast `/Game/PR/GameMode/RunGame/BP_RunPlayerController` (`GameplayStatics.GetPlayerController` _index)))
    (return _asbp_run_player_controller))
  (return _asbp_run_player_controller))

(fn `GetRunGameState`
  (returns (`AsRun Game State` :type "/Game/PR/GameMode/RunGS Object Reference"))
  (bind _asrun_gs (cast `/Game/PR/GameMode/RunGS` (`GameplayStatics.GetGameState`)))
  (return _asrun_gs))

(fn `UserConstructionScript`)