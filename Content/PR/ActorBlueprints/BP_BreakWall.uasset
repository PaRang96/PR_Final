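; BP_BreakWall is a breakable wall that a running character smashes with its attack for points.
; On the server, an overlap with the character's Attack component awards 50 points through BP_RunPlayerState.
; It then fires a RadialForce impulse, plays a collapse sound at its location and destroys itself.
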(event `self.StaticMesh.OnComponentBeginOverlap`
  (params (OverlappedComponent :type "PrimitiveComponent Object Reference") (OtherActor :type "Actor Object Reference") (OtherComp :type "PrimitiveComponent Object Reference") (OtherBodyIndex :type Integer) (bFromSweep :type Boolean) (SweepResult :type "HitResult Structure (by ref)"))
  (`/Engine/EditorBlueprintResources/ActorMacros.Switch Has Authority`
    (:`Authority`
      (bind _asinherit_run_character (cast `/Game/PR/PlayerCharacter/InheritRunCharacter` OtherActor))
      (if (== (`/RunCharacter/ProjectRun/PlayerCharacter/RunCharacter.Attack` _asinherit_run_character) OtherComp)
        (bind _asbp_run_player_state (cast `/Game/PR/GameMode/RunGame/BP_RunPlayerState` (`Pawn.PlayerState` _asinherit_run_character)))
        (`/Game/PR/GameMode/RunGame/BP_RunPlayerState.AddPoint` _asbp_run_player_state 50)
        (`RadialForceComponent.FireImpulse` (`self.RadialForce`))
        (`GameplayStatics.PlaySoundAtLocation` "/Game/StarterContent/Audio/Collapse_Cue.Collapse_Cue" (`self.K2_GetActorLocation`) (struct) 1.0 1.0 0.0 null null null)
        (`self.K2_DestroyActor`)))))

(fn `UserConstructionScript`)