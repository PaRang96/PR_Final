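; BP_MovingWall is a wall actor whose static mesh rotates in yaw from the start of play.
; A PlayRate timeline's curve, scaled by Speed, continually sets the play rate of a Rotation timeline, whose curve drives the mesh's relative yaw.
; The mesh's hit event is empty, and an authority-only launch of InheritRunCharacter is left disconnected, so it never runs.
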(event `self.ReceiveBeginPlay`
  (bind (_direction `_새_트랙_0`) (`Timeline|PlayRate`)
    (:`Update`
      (`TimelineComponent.SetPlayRate` (`self.Rotation`) (* `_새_트랙_0` (`self.Speed`)))
      (bind (_direction_2 `_새_트랙_0_2`) (`Timeline|Rotation`)
        (:`Update`
          (`SceneComponent.K2_SetRelativeRotation` (`self.StaticMesh`) (`KismetMathLibrary.MakeRotator` 0.0 0.0 `_새_트랙_0_2`) false false))))))

(event `self.StaticMesh.OnComponentHit`
  (params (HitComponent :type "PrimitiveComponent Object Reference") (OtherActor :type "Actor Object Reference") (OtherComp :type "PrimitiveComponent Object Reference") (NormalImpulse :type "Vector Structure") (Hit :type "HitResult Structure (by ref)")))

(fn `UserConstructionScript`)