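; Portal ring actor that teleports any InheritRunCharacter entering its Box to a hard-coded world location, on authority only.
; On BeginPlay, a PlayRate timeline scales the spinner timeline's speed by SpinnerSpeed and calls its PlayFromStart on every update.
; The spinner timeline drives the Propeller's yaw.
; An up-down timeline for the Ring gets the same rate but is never played, and its update logic is unconnected.
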(event `self.ReceiveBeginPlay`
  (bind (_direction _speed) (`Timeline|PlayRate`)
    (:`Update`
      (`TimelineComponent.SetPlayRate` (`self.SpinnerRotate`) (* _speed (`self.Spinner Speed`)))
      (`TimelineComponent.SetPlayRate` (`self.UpDowmTimeLine`) (* _speed (`self.Spinner Speed`)))
      (bind (_direction_2 _rotation) (`Timeline|SpinnerRotate` :!via `PlayFromStart`)
        (:`Update`
          (`SceneComponent.K2_SetRelativeRotation` (`self.Propeller`) (`KismetMathLibrary.MakeRotator` 0.0 0.0 _rotation) false false))))))

(event `self.Box.OnComponentBeginOverlap`
  (params (OverlappedComponent :type "PrimitiveComponent Object Reference") (OtherActor :type "Actor Object Reference") (OtherComp :type "PrimitiveComponent Object Reference") (OtherBodyIndex :type Integer) (bFromSweep :type Boolean) (SweepResult :type "HitResult Structure (by ref)"))
  (`/Engine/EditorBlueprintResources/ActorMacros.Switch Has Authority`
    (:`Authority`
      (bind _asinherit_run_character (cast `/Game/PR/PlayerCharacter/InheritRunCharacter` OtherActor))
      (`self.K2_SetActorLocation` _asinherit_run_character (140.0 50.0 5500.0) false false))))

(fn `UserConstructionScript`)