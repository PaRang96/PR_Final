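; BP_Goal is the goal actor that records the finishing order of players in a run.
; On the server, a character capsule overlapping its Cube adds the player's controller and state to ranking arrays, then passes the array index to the PlayerState's UpdateRank.
; The controller array's length sets replicated FinishedPlayerNum, whose OnRep prints the count and calls ReqFinishPlayer on player controllers, looping by the GameMode's player count.
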(event `self.Cube.OnComponentBeginOverlap`
  (params (OverlappedComponent :type "PrimitiveComponent Object Reference") (OtherActor :type "Actor Object Reference") (OtherComp :type "PrimitiveComponent Object Reference") (OtherBodyIndex :type Integer) (bFromSweep :type Boolean) (SweepResult :type "HitResult Structure (by ref)"))
  (bind _playerrankingcontroller (`self.PlayerRankingController`))
  (`/Engine/EditorBlueprintResources/ActorMacros.Switch Has Authority`
    (:`Authority`
      (bind _asinherit_run_character (cast `/Game/PR/PlayerCharacter/InheritRunCharacter` OtherActor))
      (if (== (`Character.CapsuleComponent` _asinherit_run_character) OtherComp)
        (bind _asbp_run_player_controller (cast `/Game/PR/GameMode/RunGame/BP_RunPlayerController` (`Pawn.GetController` _asinherit_run_character)))
        (bind _returnvalue (`KismetArrayLibrary.Array_AddUnique` _playerrankingcontroller _asbp_run_player_controller))
        (bind _asbp_run_player_state (cast `/Game/PR/GameMode/RunGame/BP_RunPlayerState` (`Controller.PlayerState` _asbp_run_player_controller)))
        (set `self.FinishedPlayerNum` (`KismetArrayLibrary.Array_Length` _playerrankingcontroller))
        (bind _asbp_run_player_state_2 (cast `/Game/PR/GameMode/RunGame/BP_RunPlayerState` (`Pawn.PlayerState` _asinherit_run_character)))
        (`KismetArrayLibrary.Array_AddUnique` (`self.PlayerRankingState`) _asbp_run_player_state_2)
        (`/Game/PR/GameMode/RunGame/BP_RunPlayerState.UpdateRank` _asbp_run_player_state _returnvalue)))))

(fn `OnRep_FinishedPlayerNum`
  (bind _finishedplayernum (`self.FinishedPlayerNum`))
  (`KismetSystemLibrary.PrintString` (`KismetStringLibrary.Conv_IntToString` _finishedplayernum) true true (struct :`R` 0.445487 :`G` 1.0 :`B` 0.796051 :`A` 1.0) 60.0)
  (bind _returnvalue (`GameModeBase.GetNumPlayers` (`GameplayStatics.GetGameMode`)))
  (for _index (range _returnvalue)
    (bind _asbp_run_player_controller (cast `/Game/PR/GameMode/RunGame/BP_RunPlayerController` (`GameplayStatics.GetPlayerController` _index)))
    (`/Game/PR/GameMode/RunGame/BP_RunPlayerController.ReqFinishPlayer` _asbp_run_player_controller _finishedplayernum)))

(fn `UserConstructionScript`)